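; FishBase_BP is a fish world object, apparently a base class, that holds a fish ID and its radar icon.
; SetFishId stores the ID, finds its FishRecorder entry through the GameManagerBP game instance's config manager, and caches that entry's radar icon.
; BeginPlay calls SetFishId with a hardcoded ID, and getters expose both the ID and the icon.
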(event `self.ReceiveBeginPlay`
  (`self.SetFishId` 4))

(fn `GetFishId`
  (returns (fishId :type Integer))
  (return (`self.fishId`)))

(fn `GetRadarIcon`
  (returns (radarIcon :type Integer))
  (return (`self.radarIcon`)))

(fn `SetFishId`
  (params (fishId :type Integer))
  (set `self.fishId` fishId)
  (bind _asgame_manager_bp (cast `/Game/GameContent/Blueprint/GameManagerBP` (`GameplayStatics.GetGameInstance`)))
  (bind _returnvalue (`GameManager.GetConfigManager` _asgame_manager_bp))
  (bind _returnvalue_2 (`ConfigManager.GetConfigByName` _returnvalue "/Script/FinalFantasyFishGame.FishRecorder"))
  (bind _asfish_recorder (cast `FishRecorder` (`BlueprintMapLibrary.Map_Find` _returnvalue_2 (`self.fishId`))))
  (bind _returnvalue_3 (`FishRecorder.GetRadarIcon` _asfish_recorder))
  (set `self.radarIcon` _returnvalue_3))

(fn `UserConstructionScript`)