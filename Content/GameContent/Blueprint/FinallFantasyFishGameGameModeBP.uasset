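; Game mode for a fish game that boots the session and switches between start screen, gameplay and menu states.
; On BeginPlay it initializes the GameManagerBP game instance, loads user data, creates the start, common and menu widgets, and disables character input.
; EnterGameState and EnterMenuState toggle character input and widget visibility while tracking state flags.
; Tick is forwarded manually to the game instance.
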(event `self.ReceiveBeginPlay`
  (`self.InitInfo`)
  (`self.InitUI`)
  (set `PlayerController.bShowMouseCursor` true (`GameplayStatics.GetPlayerController` 0))
  (`self.DisableInput` (`GameplayStatics.GetPlayerCharacter` 0) (`GameplayStatics.GetPlayerController` 0)))

(event `self.ReceiveTick`
  (params (DeltaSeconds :type "Float (single-precision)"))
  (`GameManager.Tick` (`self.gameManagerBP`) DeltaSeconds))

(fn `EnterGameState`
  (set `self.haveEnterGame` true)
  (set `self.inMenuState` false)
  (`self.EnableInput` (`GameplayStatics.GetPlayerCharacter` 0) (`GameplayStatics.GetPlayerController` 0))
  (`Widget.SetVisibility` (`self.commonUI`) "Visible")
  (`Widget.SetVisibility` (`self.menuUI`) "Hidden"))

(fn `EnterMenuState`
  (set `self.inMenuState` true)
  (`self.DisableInput` (`GameplayStatics.GetPlayerCharacter` 0) (`GameplayStatics.GetPlayerController` 0))
  (`Widget.SetVisibility` (`self.commonUI`) "Hidden")
  (`Widget.SetVisibility` (`self.menuUI`) "Visible"))

(fn `GetHaveEnterGame`
  (returns (haveEnterGame :type Boolean))
  (return (`self.haveEnterGame`)))

(fn `GetInMenuState`
  (returns (isMenuState :type Boolean))
  (return (`self.inMenuState`)))

(fn `InitInfo`
  (bind _asgame_manager_bp (cast `/Game/GameContent/Blueprint/GameManagerBP` (`GameplayStatics.GetGameInstance`)))
  (bind _output_get (set `self.gameManagerBP` _asgame_manager_bp))
  (`|ExecutionSequence`
    (:`then_0`
      (`GameManager.InitAll` _output_get))
    (:`then_1`
      (`GameManager.LoadUserData` _output_get))))

(fn `InitUI`
  (`|ExecutionSequence`
    (:`then_0`
      (bind _returnvalue (`|CreateWidget` "/Game/GameContent/UI/StartGameUI.StartGameUI_C"))
      (`UserWidget.AddToViewport` _returnvalue 0))
    (:`then_1`
      (bind _returnvalue_2 (`|CreateWidget` "/Game/GameContent/UI/CommonUI.CommonUI_C"))
      (`UserWidget.AddToViewport` _returnvalue_2 0)
      (bind _output_get (set `self.commonUI` _returnvalue_2))
      (`Widget.SetVisibility` _output_get "Hidden"))
    (:`then_2`
      (bind _returnvalue_3 (`|CreateWidget` "/Game/GameContent/UI/MeunUI.MeunUI_C"))
      (`UserWidget.AddToViewport` _returnvalue_3 0)
      (bind _output_get_2 (set `self.menuUI` _returnvalue_3))
      (`Widget.SetVisibility` _output_get_2 "Hidden"))))

(fn `UserConstructionScript`)