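; Game manager Blueprint that tracks spawned fish and an InFishing flag for the fishing gameplay.
; ExecuteActionBPEvent parses text commands, dispatching addfish to spawn a FishBase_BP at X/Y and clearfish to remove fish.
; AddFish stores each actor in FishList but ignores its type argument.
; RemoveAllFish destroys those actors without clearing the list, and RemoveFishByType is an empty stub.
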(event `self.ExecuteAction_BPEvent`
  (params (actionString :type String))
  (bind _returnvalue (`KismetStringLibrary.ParseIntoArray` actionString))
  (bind _actionstringlist (`self.actionStringList`))
  (bind _actionstringlist_2 (`self.actionStringList`))
  (bind _output (`|GetArrayItem` (`self.actionStringList`)))
  (set `self.actionStringList` _returnvalue)
  (if (> (`KismetArrayLibrary.Array_Length` _returnvalue) 0)
    (`|ExecutionSequence`
      (:`then_0`
        ;[1 1 1] 向指定位置添加指定类型的鱼：addfish type positionx positiony
        (if (`KismetStringLibrary.EqualEqual_StrStr` _output "addfish")
          (if (>= (`KismetArrayLibrary.Array_Length` _actionstringlist_2) 4)
            (`self.AddFish` (`KismetStringLibrary.Conv_StringToInt` (`|GetArrayItem` _actionstringlist_2 1)) (`KismetStringLibrary.Conv_StringToDouble` (`|GetArrayItem` _actionstringlist_2 2)) (`KismetStringLibrary.Conv_StringToDouble` (`|GetArrayItem` _actionstringlist_2 3)))
            (else
              (`KismetSystemLibrary.PrintString` "指令的参数数量不匹配：addfish type positionx positiony")))))
      (:`then_1`
        ;[1 1 1] 清除所有鱼 clearfish type(不填代表删除所有)
        (if (`KismetStringLibrary.EqualEqual_StrStr` _output "clearfish")
          (if (> (`KismetArrayLibrary.Array_Length` _actionstringlist) 1)
            (`self.RemoveFishByType` (`KismetStringLibrary.Conv_StringToInt` (`|GetArrayItem` _actionstringlist 1)))
            (else
              (`self.RemoveAllFish`))))))))

(fn `AddFish`
  (params (fishType :type Integer) (x :type "Float (double-precision)") (y :type "Float (double-precision)"))
  (bind _returnvalue (`|SpawnActorFromClass` "/Game/GameContent/Blueprint/WorldObjectBP/Fish/FishBase_BP.FishBase_BP_C" (`KismetMathLibrary.MakeTransform` (`KismetMathLibrary.MakeVector` x y)) "Undefined" "OverrideRootScale" null null))
  (`KismetArrayLibrary.Array_Add` (`self.fishList`) _returnvalue))

(fn `EnterFish`
  (set `self.inFishing` true))

(fn `ExitFish`
  (set `self.inFishing` false))

(fn `GetFishList`
  (returns (NewParam :type "Array of /Game/GameContent/Blueprint/WorldObjectBP/Fish/FishBase_BP Object Reference"))
  (return (`self.fishList`)))

(fn `RemoveAllFish`
  (for _array_element (`self.fishList`)
    (`Actor.K2_DestroyActor` _array_element)))

(fn `RemoveFishByType`
  (params (fishType :type Integer)))