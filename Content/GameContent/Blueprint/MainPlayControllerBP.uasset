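; MainPlayControllerBP is the main player controller that lets the player toggle the menu during play.
; On BeginPlay it casts the game mode to FinallFantasyFishGameGameModeBP and caches it.
; Pressing ShowOrHideMenuUI, once the game has been entered, checks the game mode's menu state and calls EnterGameState or EnterMenuState, leaving the state logic to the game mode.
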(event `self.ReceiveBeginPlay`
  (bind _asfinall_fantasy_fish_game_game_mode_bp (cast `/Game/GameContent/Blueprint/FinallFantasyFishGameGameModeBP` (`GameplayStatics.GetGameMode`)))
  (set `self.gameModeBP` _asfinall_fantasy_fish_game_game_mode_bp))

(event `InputAction|ShowOrHideMenuUI`
  (params (Key :type "Key Structure"))
  (bind _gamemodebp (`self.gameModeBP`))
  (:`Pressed`
    (bind _haveentergame (`/Game/GameContent/Blueprint/FinallFantasyFishGameGameModeBP.GetHaveEnterGame` (`self.gameModeBP`)))
    (if _haveentergame
      (bind _ismenustate (`/Game/GameContent/Blueprint/FinallFantasyFishGameGameModeBP.GetInMenuState` _gamemodebp))
      (if _ismenustate
        (`/Game/GameContent/Blueprint/FinallFantasyFishGameGameModeBP.EnterGameState` _gamemodebp)
        (else
          (`/Game/GameContent/Blueprint/FinallFantasyFishGameGameModeBP.EnterMenuState` _gamemodebp))))))

(fn `UserConstructionScript`)